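; CubePawn is a scoring cube target that explodes when hit.
; A hit on the Cube component spawns Blueprint_Effect_Explosion at its transform, destroys the component and adds TargetScore through AddTargetPoints on FirstPersonGameMode.
; The spawned effect is stored in Explosion, and an Explosion EndPlay event destroys the pawn itself.
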(event OnComponentHit(Cube)
  (params (HitComponent :type Primitive%20Component%20Object%20Reference) (OtherActor :type Actor%20Object%20Reference) (OtherComp :type Primitive%20Component%20Object%20Reference) (NormalImpulse :type Vector :default "0, 0, 0") (Hit :type Hit%20Result%20Structure%20%28by%20ref%29))
  (Utilities|FlowControl|Sequence
    (:then_0
      ;[1 0.01186 0] Destroy CubePawn
      (bind _returnvalue (Game|SpawnActorfromClass "/Game/StarterContent/Blueprints/Blueprint_Effect_Explosion.Blueprint_Effect_Explosion_C" (Transformation|GetWorldTransform (Variables|Default|GetCube)) "Undefined" 0 0))
      (Variables|Default|SetExplosion _returnvalue))
    (:then_1
      (Components|DestroyComponent (Variables|Default|GetCube)))
    (:then_2
      ;[0.3001 1 0.1914] Call AddScore Function
      (bind _asfirst_person_game_mode (Utilities|Casting|CastToFirstPersonGameMode (Game|GetGameMode)))
      (Default|AddTargetPoints _asfirst_person_game_mode (Variables|Default|GetTargetScore)))))

(event OnEndPlay(Explosion)
  (params (Actor :type Actor%20Object%20Reference) (EndPlayReason :type EEndPlayReason%20Enum :default "Destroyed"))
  ;[1 0.01186 0] Destroy CubePawn
  (Actor|DestroyActor))

(fn ConstructionScript)